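; Player character for Astrobot, with Enhanced Input move, look, jump-to-hover and basic attack; pause is a print stub.
; Tick drives the spring arm: a ground sphere trace sets pivot height, held while falling, and a camera line trace adjusts arm length.
; Hover retunes jump hold time and Z velocity; the throttled attack only line-traces and prints the hit.
; Overlapped collectables are passed to BP_UIManager's inventory.
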(event `self.ReceiveTick`
  (params (DeltaSeconds :type "Float (single-precision)"))
  (bind (_target_camera_pivot_x _target_camera_pivot_y _target_camera_pivot_z) (`KismetMathLibrary.BreakVector` (`self.Target Camera Pivot`)))
  (bind _springarm (`self.SpringArm`))
  (bind _returnvalue (`SceneComponent.K2_GetComponentLocation` (`self.Mesh`)))
  (bind _returnvalue_2 (`SceneComponent.K2_GetComponentLocation` (`self.Mesh`)))
  (bind (_returnvalue_x _returnvalue_y) (`KismetMathLibrary.BreakVector` (`SceneComponent.K2_GetComponentLocation` (`self.Mesh`))))
  (bind (_returnvalue_x_2 _returnvalue_y_2) (`KismetMathLibrary.BreakVector` (`SceneComponent.K2_GetComponentLocation` (`self.Mesh`))))
  ;[1 1 1] LineTrace Camera
  (if (`NavMovementComponent.IsFalling` (`self.CharacterMovement`))
    (`SceneComponent.K2_SetWorldLocation` (`self.SpringArm`) (`KismetMathLibrary.MakeVector` _returnvalue_x _returnvalue_y _target_camera_pivot_z) false false)
    (else
      (bind (_outhit _returnvalue_3) (`KismetSystemLibrary.SphereTraceSingle` _returnvalue (+ (* (* (`SceneComponent.GetUpVector` (`self.CapsuleComponent`)) -1.0) 1000.0) _returnvalue) 25.0 "TraceTypeQuery1"))
      (if _returnvalue_3
        (bind _output_get (set `self.Target Camera Pivot` (+ (`.Location` (`GameplayStatics.BreakHitResult` _outhit)) (0.0 0.0 10.0))))
        (bind (_returnvalue_x_3 _returnvalue_y_3 _returnvalue_z) (`KismetMathLibrary.BreakVector` (`KismetMathLibrary.VInterpTo` (`SceneComponent.RelativeLocation` (`self.SpringArm`)) _output_get (`GameplayStatics.GetWorldDeltaSeconds`) 1.0)))
        (`SceneComponent.K2_SetWorldLocation` (`self.SpringArm`) (`KismetMathLibrary.MakeVector` _returnvalue_x_2 _returnvalue_y_2 _returnvalue_z) false false)
        ;[1 1 1] Camera Forward Linetrace
        (bind _outhit_2 (`KismetSystemLibrary.LineTraceSingle` :`Start` _returnvalue_2 :`End` (+ _returnvalue_2 (* (`SceneComponent.GetForwardVector` (`self.Camera`)) -1000.0)) :`TraceChannel` "TraceTypeQuery1" :`bIgnoreSelf` false))
        (bind (_bblockinghit _binitialoverlap _time _distance _location _impactpoint _normal _impactnormal _physmat _hitactor) (`GameplayStatics.BreakHitResult` _outhit_2))
        (if _bblockinghit
          (if (!= _hitactor self)
            (set `SpringArmComponent.TargetArmLength` (`KismetMathLibrary.VSize` (- _location (`self.K2_GetActorLocation`))) _springarm))
          (else
            (set `SpringArmComponent.TargetArmLength` 700.0 _springarm)))))))

(event `self.ReceiveBeginPlay`
  ;[1 1 1] Getting Mapping Context
  (bind _asplayer_controller (cast `PlayerController` (`self.GetController`)))
  (bind _returnvalue (pcsubsystem `EnhancedInputLocalPlayerSubsystem` _asplayer_controller))
  (`/Engine/EditorBlueprintResources/StandardMacros.IsValid` _returnvalue
    (:`Is Valid`
      (`EnhancedInputSubsystemInterface.AddMappingContext` _returnvalue "/Game/Characters/Astrobot/ControlMapping/AstrobotMapping.AstrobotMapping" 0 (struct)))))

(event `EnhancedInput|/Game/Characters/Astrobot/ControlMapping/Actions/IA_BasicAttack`
  (params (ActionValue :type Boolean) (ElapsedSeconds :type "Float (double-precision)") (TriggeredSeconds :type "Float (double-precision)") (InputAction :type "InputAction Object Reference" :default "/Game/Characters/Astrobot/ControlMapping/Actions/IA_BasicAttack.IA_BasicAttack"))
  ;[1 1 1] Basic Attack
  (:`Triggered`
    (if (not (`self.AbilityActive?`))
      (`/Engine/EditorBlueprintResources/StandardMacros.DoOnce` false :!label _label
        (:`Completed`
          (`self.BasicAttack`)
          (`KismetSystemLibrary.Delay` 0.3)
          (goto _label :!via `Reset`))))))

(event `EnhancedInput|/Game/Characters/Astrobot/ControlMapping/Actions/IA_AbilityLeft`
  (params (ActionValue :type Boolean) (ElapsedSeconds :type "Float (double-precision)") (TriggeredSeconds :type "Float (double-precision)") (InputAction :type "InputAction Object Reference" :default "/Game/Characters/Astrobot/ControlMapping/Actions/IA_AbilityLeft.IA_AbilityLeft")))

(event `EnhancedInput|/Game/Characters/Astrobot/ControlMapping/Actions/IA_LookMovement`
  (params (ActionValue :type "Vector2D Structure") (ElapsedSeconds :type "Float (double-precision)") (TriggeredSeconds :type "Float (double-precision)") (InputAction :type "InputAction Object Reference" :default "/Game/Characters/Astrobot/ControlMapping/Actions/IA_LookMovement.IA_LookMovement"))
  ;[1 1 1] Look Movement
  (:`Triggered`
    (`self.AddControllerYawInput` ActionValue_X)
    (`self.AddControllerPitchInput` ActionValue_Y)))

(event `EnhancedInput|/Game/Characters/Astrobot/ControlMapping/Actions/IA_Pause`
  (params (ActionValue :type Boolean) (ElapsedSeconds :type "Float (double-precision)") (TriggeredSeconds :type "Float (double-precision)") (InputAction :type "InputAction Object Reference" :default "/Game/Characters/Astrobot/ControlMapping/Actions/IA_Pause.IA_Pause"))
  ;[1 0 0] Pause Menu
  (:`Triggered`
    (`KismetSystemLibrary.PrintString` "Paused")))

(event `EnhancedInput|/Game/Characters/Astrobot/ControlMapping/Actions/IA_Movement`
  (params (ActionValue :type "Vector2D Structure") (ElapsedSeconds :type "Float (double-precision)") (TriggeredSeconds :type "Float (double-precision)") (InputAction :type "InputAction Object Reference" :default "/Game/Characters/Astrobot/ControlMapping/Actions/IA_Movement.IA_Movement"))
  (bind (_returnvalue_roll _returnvalue_pitch _returnvalue_yaw) (`KismetMathLibrary.BreakRotator` (`self.GetControlRotation`)))
  (bind (_returnvalue_roll_2 _returnvalue_pitch_2 _returnvalue_yaw_2) (`KismetMathLibrary.BreakRotator` (`self.GetControlRotation`)))
  ;[1 1 1] Character Movement
  (:`Triggered`
    (`self.AddMovementInput` (`KismetMathLibrary.GetRightVector` (`KismetMathLibrary.MakeRotator` _returnvalue_roll_2 0.0 _returnvalue_yaw_2)) ActionValue_X)
    (`self.AddMovementInput` (`KismetMathLibrary.GetForwardVector` (`KismetMathLibrary.MakeRotator` 0.0 0.0 _returnvalue_yaw)) ActionValue_Y)))

(event `EnhancedInput|/Game/Characters/Astrobot/ControlMapping/Actions/IA_Jump_Hover`
  (params (ActionValue :type Boolean) (ElapsedSeconds :type "Float (double-precision)") (TriggeredSeconds :type "Float (double-precision)") (InputAction :type "InputAction Object Reference" :default "/Game/Characters/Astrobot/ControlMapping/Actions/IA_Jump_Hover.IA_Jump_Hover"))
  (bind _returnvalue (>= (`self.JumpCurrentCount`) 1))
  ;[1 0 0] Jump/Hover
  (:`Started`
    (`self.Jump`)
    (if _returnvalue
      (`|ExecutionSequence`
        (:`then_0`
          (set `self.JumpMaxHoldTime` 1.0)
          (if (and _returnvalue (`self.CanJump`))
            _))
        (:`then_1`
          (set `CharacterMovementComponent.JumpZVelocity` 100.0 (`self.CharacterMovement`))))))
  (:`Completed`
    (`self.StopJumping`)
    (`|ExecutionSequence`
      (:`then_0`
        (set `self.JumpMaxHoldTime` 0.0))
      (:`then_1`
        (set `CharacterMovementComponent.JumpZVelocity` 1500.0 (`self.CharacterMovement`))))))

(event `self.CapsuleComponent.OnComponentBeginOverlap`
  (params (OverlappedComponent :type "PrimitiveComponent Object Reference") (OtherActor :type "Actor Object Reference") (OtherComp :type "PrimitiveComponent Object Reference") (OtherBodyIndex :type Integer) (bFromSweep :type Boolean) (SweepResult :type "HitResult Structure (by ref)"))
  ;[1 1 1] Adds overlapping Coins and Puzzle Pieces to the Collectable Inventory
  (bind _is_collectable (message `/AstrobotCollectables/BPI_CollectableInterface.Is Collectable` OtherActor true))
  (if _is_collectable
    (bind _returnvalue (`GameplayStatics.GetActorOfClass` "/Game/UI__Design_/BP_UIManager.BP_UIManager_C"))
    (`/AstrobotCollectables/BPI_CollectableInterface.Add Coin To Player Inventory` _returnvalue false)
    (message `/AstrobotCollectables/BPI_CollectableInterface.Collect Item` OtherActor (`/Game/UI__Design_/BP_UIManager.BP_CollectableInventory` _returnvalue) false)))

(fn `BasicAttack`
  (bind _returnvalue (`SceneComponent.K2_GetComponentLocation` (`self.Mesh`)))
  (bind _outhit (`KismetSystemLibrary.LineTraceSingle` :`Start` (+ _returnvalue (0.0 0.0 2.0)) :`End` (+ (* (`SceneComponent.GetForwardVector` (`self.Mesh`)) 250.0) _returnvalue) :`TraceChannel` "TraceTypeQuery1" :`DrawDebugType` "ForDuration"))
  (`KismetSystemLibrary.PrintString` (`KismetSystemLibrary.GetDisplayName` (`.HitActor` (`GameplayStatics.BreakHitResult` _outhit)))))

(fn `UserConstructionScript`)