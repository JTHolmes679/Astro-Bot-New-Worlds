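; BP_AstrobotPlayer2Character is the second-player Astrobot character, layering startup and UI input on its parent class.
; On BeginPlay it runs the parent logic, then calls CreatePlayer with an automatic controller ID to add a local player.
; Enhanced Input actions for closing the tutorial and pausing each look up BP_UIManager in the world, calling its HUD right prompt and pause menu respectively.
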(event `self.ReceiveBeginPlay`
  (`parent.ReceiveBeginPlay`)
  (`GameplayStatics.CreatePlayer` -1))

(event `EnhancedInput|/Game/Characters/Astrobot/ControlMapping/Actions/IA_CloseTutorial`
  (params (ActionValue :type Boolean) (ElapsedSeconds :type "Float (double-precision)") (TriggeredSeconds :type "Float (double-precision)") (InputAction :type "InputAction Object Reference" :default "/Game/Characters/Astrobot/ControlMapping/Actions/IA_CloseTutorial.IA_CloseTutorial"))
  ;[1 1 1] Close tutorial
  (:`Triggered`
    (bind _returnvalue (`GameplayStatics.GetActorOfClass` "/Game/UI__Design_/BP_UIManager.BP_UIManager_C"))
    (`/Game/UI__Design_/WBP_HUD.RightPrompt` (`/Game/UI__Design_/BP_UIManager.HUD` _returnvalue))))

(event `EnhancedInput|/Game/Characters/Astrobot/ControlMapping/Actions/IA_Pause`
  (params (ActionValue :type Boolean) (ElapsedSeconds :type "Float (double-precision)") (TriggeredSeconds :type "Float (double-precision)") (InputAction :type "InputAction Object Reference" :default "/Game/Characters/Astrobot/ControlMapping/Actions/IA_Pause.IA_Pause"))
  ;[1 1 1] Open pause menu
  (:`Triggered`
    (bind _returnvalue (`GameplayStatics.GetActorOfClass` "/Game/UI__Design_/BP_UIManager.BP_UIManager_C"))
    (`/Game/UI__Design_/WBP_Pause.PauseMenu` (`/Game/UI__Design_/BP_UIManager.Pause` _returnvalue))))

(fn `UserConstructionScript`
  (`parent.UserConstructionScript`))