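; Friendly Astrobot character Blueprint that reacts when the player approaches, with early debug-level behavior.
; When the player character overlaps its Box, it prints a greeting and plays a walk animation once on the Mesh.
; A BasicAttack function, not called within this Blueprint, runs a short debug-drawn visibility line trace along the mesh's forward vector and prints the hit actor's name, without applying damage.
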(event `self.Box.OnComponentBeginOverlap`
  (params (OverlappedComponent :type "PrimitiveComponent Object Reference") (OtherActor :type "Actor Object Reference") (OtherComp :type "PrimitiveComponent Object Reference") (OtherBodyIndex :type Integer) (bFromSweep :type Boolean) (SweepResult :type "HitResult Structure (by ref)"))
  (if (== OtherActor (`GameplayStatics.GetPlayerCharacter` 0))
    (`KismetSystemLibrary.PrintString` "Hello")
    (`SkeletalMeshComponent.PlayAnimation` (`self.Mesh`) "/Game/Characters/Astrobot/Animations/normal_walk.normal_walk" false)))

(fn `BasicAttack`
  (bind _returnvalue (`SceneComponent.K2_GetComponentLocation` (`self.Mesh`)))
  (bind _outhit (`KismetSystemLibrary.LineTraceSingle` :`Start` (+ _returnvalue (0.0 0.0 2.0)) :`End` (+ (* (`SceneComponent.GetForwardVector` (`self.Mesh`)) 250.0) _returnvalue) :`TraceChannel` "TraceTypeQuery1" :`DrawDebugType` "ForDuration"))
  (`KismetSystemLibrary.PrintString` (`KismetSystemLibrary.GetDisplayName` (`.HitActor` (`GameplayStatics.BreakHitResult` _outhit)))))

(fn `UserConstructionScript`)