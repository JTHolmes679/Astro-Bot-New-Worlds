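; BP_overcharge_ball is an actor that emits beam effects from around itself to nearby blocking surfaces, apparently as electric-style arcs.
; Each Tick, Updatetracers checks a cooldown, then line traces from a random point at Minradius.
; The trace's End is unset, as the Maxradius calculation is unconnected.
; On a hit, it spawns an attached, auto-destroying Niagara system, passing start point, normal-offset impact point and impact normal.
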(event `self.ReceiveTick`
  (params (DeltaSeconds :type "Float (single-precision)"))
  (`self.updatetracers`))

(fn `updatetracers`
  (locals (randomdirection :type "Vector Structure" :default (0.0 0.0 0.0)) (impactoffset :type "Float (double-precision)" :default 1.0))
  (bind _returnvalue (* (`local.randomdirection`) (`self.minradius`)))
  ;[1 1 1] Check Cooldown
  (if (>= (- (`GameplayStatics.GetTimeSeconds`) (`self.lasttrace`)) (`self.tracecooldown`))
    ;[1 1 1] Trace
    (set `local.randomdirection` (`KismetMathLibrary.RandomUnitVector`))
    (bind _outhit (`KismetSystemLibrary.LineTraceSingle` :`Start` (+ (`self.K2_GetActorLocation`) _returnvalue) :`TraceChannel` "TraceTypeQuery1" :`DrawTime` (`self.tracecooldown`)))
    ;[1 1 1] Reset trace cooldown
    (set `self.lasttrace` (`GameplayStatics.GetTimeSeconds`))
    (bind (_bblockinghit _binitialoverlap _time _distance _location _impactpoint _normal _impactnormal) (`GameplayStatics.BreakHitResult` _outhit))
    ;[1 1 1] spawn niagar system and set parameters
    (if _bblockinghit
      (bind _returnvalue_2 (`NiagaraFunctionLibrary.SpawnSystemAttached` null (`self.DefaultSceneRoot`) "None" (0.0 0.0 0.0) (struct) "KeepRelativeOffset" true))
      (`NiagaraComponent.SetVariableVec3` _returnvalue_2 "beamstartpoint" _returnvalue)
      (`NiagaraComponent.SetVariableVec3` _returnvalue_2 "beamendpoint" (+ _impactpoint (* _impactnormal (`local.impactoffset`))))
      (`NiagaraComponent.SetVariableVec3` _returnvalue_2 "impactnormal" _impactnormal))))

(fn `UserConstructionScript`)