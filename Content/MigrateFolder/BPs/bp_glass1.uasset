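; Resizable framed glass panel actor, assembled entirely in the Construction Script from FrameWidth and FrameHeight.
; Four corner pieces and four edge pieces are offset by half those dimensions to form the frame.
; Glass and edges stretch by frame size over mesh bounds, added to their current relative scale.
; Only X extents are measured: the glass's own for both its axes, the top edge's for all edges.
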(fn `UserConstructionScript`
  (bind _glassmesh (`self.glassmesh`))
  (bind _edger (`self.edgeR`))
  (bind _edgel (`self.edgeL`))
  (bind _edget (`self.edgeT`))
  (bind _frameheight (`self.FrameHeight`))
  (bind _edgeb (`self.edgeB`))
  (bind _framewidth (`self.FrameWidth`))
  (bind (_returnvalue_min _returnvalue_max) (break `Box` (`StaticMesh.GetBoundingBox` (`StaticMeshComponent.StaticMesh` _glassmesh))))
  (bind (_returnvalue_min_2 _returnvalue_max_2) (break `Box` (`StaticMesh.GetBoundingBox` (`StaticMeshComponent.StaticMesh` _edget))))
  (bind (_returnvalue_x _returnvalue_y) (`KismetMathLibrary.BreakVector` (+ (`SceneComponent.RelativeScale3D` _edgel) (`KismetMathLibrary.MakeVector` 0.0 (/ (`self.FrameHeight`) (`self.Frame Length`))))))
  (bind (_returnvalue_x_2 _returnvalue_y_2) (`KismetMathLibrary.BreakVector` (+ (`SceneComponent.RelativeScale3D` _glassmesh) (`KismetMathLibrary.MakeVector` (/ (`self.FrameWidth`) (`self.glass length`)) (/ (`self.FrameHeight`) (`self.glass length`))))))
  (bind _returnvalue_x_3 (`KismetMathLibrary.BreakVector` (+ (`SceneComponent.RelativeScale3D` _edget) (`KismetMathLibrary.MakeVector` (/ (`self.FrameWidth`) (`self.Frame Length`))))))
  (bind _returnvalue_x_4 (`KismetMathLibrary.BreakVector` (+ (`SceneComponent.RelativeScale3D` _edgeb) (`KismetMathLibrary.MakeVector` (/ (`self.FrameWidth`) (`self.Frame Length`))))))
  (bind (_returnvalue_x_5 _returnvalue_y_3) (`KismetMathLibrary.BreakVector` (+ (`SceneComponent.RelativeScale3D` _edger) (`KismetMathLibrary.MakeVector` 0.0 (/ (`self.FrameHeight`) (`self.Frame Length`))))))
  (bind _returnvalue_x_6 (`KismetMathLibrary.BreakVector` (- _returnvalue_max _returnvalue_min)))
  (bind _returnvalue_x_7 (`KismetMathLibrary.BreakVector` (- _returnvalue_max_2 _returnvalue_min_2)))
  (`|ExecutionSequence`
    (:`then_0`
      (`SceneComponent.K2_SetRelativeLocation` (`self.BL`) (`KismetMathLibrary.MakeVector` (/ (`self.FrameWidth`) 2.0) (* (/ (`self.FrameHeight`) 2.0) -1.0)) false false))
    (:`then_1`
      (`SceneComponent.K2_SetRelativeLocation` (`self.BR`) (`KismetMathLibrary.MakeVector` (* (/ (`self.FrameWidth`) 2.0) -1.0) (* (/ (`self.FrameHeight`) 2.0) -1.0)) false false))
    (:`then_2`
      (`SceneComponent.K2_SetRelativeLocation` (`self.TR`) (`KismetMathLibrary.MakeVector` (* (/ (`self.FrameWidth`) 2.0) -1.0) (/ (`self.FrameHeight`) 2.0)) false false))
    (:`then_3`
      (`SceneComponent.K2_SetRelativeLocation` (`self.TL`) (`KismetMathLibrary.MakeVector` (/ (`self.FrameWidth`) 2.0) (/ (`self.FrameHeight`) 2.0)) false false))
    (:`then_4`
      (set `self.glass length` _returnvalue_x_6)
      (`SceneComponent.SetRelativeScale3D` _glassmesh (`KismetMathLibrary.MakeVector` _returnvalue_x_2 _returnvalue_y_2 1.0)))
    (:`then_5`
      (`SceneComponent.K2_SetRelativeLocation` _edget (`KismetMathLibrary.MakeVector` 0.0 (* _frameheight -0.5)) false false)
      (`SceneComponent.K2_SetRelativeLocation` _edgeb (`KismetMathLibrary.MakeVector` 0.0 (* _frameheight 0.5)) false false)
      (`SceneComponent.K2_SetRelativeLocation` _edger (`KismetMathLibrary.MakeVector` (* _framewidth 0.5)) false false)
      (`SceneComponent.K2_SetRelativeLocation` _edgel (`KismetMathLibrary.MakeVector` (* _framewidth -0.5)) false false)
      (set `self.Frame Length` _returnvalue_x_7)
      (`SceneComponent.SetRelativeScale3D` _edget (`KismetMathLibrary.MakeVector` _returnvalue_x_3 1.0 1.0))
      (`SceneComponent.SetRelativeScale3D` _edgeb (`KismetMathLibrary.MakeVector` _returnvalue_x_4 1.0 1.0))
      (`SceneComponent.SetRelativeScale3D` _edger (`KismetMathLibrary.MakeVector` 1.0 _returnvalue_y_3 1.0))
      (`SceneComponent.SetRelativeScale3D` _edgel (`KismetMathLibrary.MakeVector` 1.0 _returnvalue_y 1.0)))))