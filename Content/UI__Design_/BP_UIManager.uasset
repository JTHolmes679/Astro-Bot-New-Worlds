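; BP_UIManager creates and holds the game's main UI widgets and relays collectable and readiness events to them.
; After a short delay on BeginPlay it adds the HUD, pause, friend-rescued and ready widgets to the viewport.
; Coin pickups update both HUD and pause widgets, while rescued friends go to the collectable inventory.
; A ready counter drives the ready widget's text and opacity; the getter functions return only default values.
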(event `self.ReceiveBeginPlay`
  (`KismetSystemLibrary.Delay` 0.2)
  (bind _returnvalue (`|CreateWidget` "/Game/UI__Design_/WBP_HUD.WBP_HUD_C"))
  (`UserWidget.AddToViewport` _returnvalue 0)
  (set `self.HUD` _returnvalue)
  (bind _returnvalue_2 (`|CreateWidget` "/Game/UI__Design_/WBP_Pause.WBP_Pause_C"))
  (`UserWidget.AddToViewport` _returnvalue_2 0)
  (set `self.Pause` _returnvalue_2)
  (bind _returnvalue_3 (`|CreateWidget` "/Game/UI__Design_/WBP_FriendRescued.WBP_FriendRescued_C"))
  (`UserWidget.AddToViewport` _returnvalue_3 0)
  (set `self.Friend Collected` _returnvalue_3)
  (bind _returnvalue_4 (`|CreateWidget` "/Game/UI__Design_/WBP_Ready.WBP_Ready_C"))
  (`UserWidget.AddToViewport` _returnvalue_4 0)
  (bind _output_get (set `self.Ready` _returnvalue_4)))

(event `/AstrobotCollectables/BPI_CollectableInterface.Add Coin To Player Inventory`
  (params (bDebugMode :type Boolean))
  (if bDebugMode
    (`KismetSystemLibrary.PrintString` "Manager"))
  (`/Game/UI__Design_/WBP_HUD.Add Coin To Player Inventory` (`self.HUD`) bDebugMode)
  (`/Game/UI__Design_/WBP_Pause.Add Coin To Player Inventory` (`self.Pause`) false))

(event `count`
  (set `self.countReady` (+ (`self.countReady`) 1))
  (if (== (`self.countReady`) 1)
    (set `Widget.RenderOpacity` 1.0 (stale `self.ReceiveBeginPlay` _returnvalue_4))
    (set `/Game/UI__Design_/WBP_Ready.realtext` (`/Game/UI__Design_/WBP_Ready.1 in` (stale `self.ReceiveBeginPlay` _output_get)) (stale `self.ReceiveBeginPlay` _returnvalue_4))
    (elif (== (`self.countReady`) 2)
      (set `/Game/UI__Design_/WBP_Ready.realtext` (`/Game/UI__Design_/WBP_Ready.2 in` (stale `self.ReceiveBeginPlay` _returnvalue_4)) (stale `self.ReceiveBeginPlay` _returnvalue_4))
      (elif (== (`self.countReady`) 0)
        (set `/Game/UI__Design_/WBP_Ready.realtext` (`/Game/UI__Design_/WBP_Ready.realtext` (stale `self.ReceiveBeginPlay` _returnvalue_4)) (stale `self.ReceiveBeginPlay` _returnvalue_4))
        (set `Widget.RenderOpacity` 0.0 (stale `self.ReceiveBeginPlay` _output_get) :!label _label)))))

(event `countdown`
  (set `self.countReady` (- (`self.countReady`) 1))
  (if (== (`self.countReady`) 1)
    (set `Widget.RenderOpacity` 1.0 (stale `self.ReceiveBeginPlay` _returnvalue_4))
    (set `/Game/UI__Design_/WBP_Ready.realtext` (`/Game/UI__Design_/WBP_Ready.1 in` (stale `self.ReceiveBeginPlay` _returnvalue_4)) (stale `self.ReceiveBeginPlay` _returnvalue_4))
    (elif (== (`self.countReady`) 2)
      (set `/Game/UI__Design_/WBP_Ready.realtext` (`/Game/UI__Design_/WBP_Ready.2 in` (stale `self.ReceiveBeginPlay` _returnvalue_4)) (stale `self.ReceiveBeginPlay` _returnvalue_4))
      (elif (== (`self.countReady`) 0)
        (set `/Game/UI__Design_/WBP_Ready.realtext` (`/Game/UI__Design_/WBP_Ready.realtext` (stale `self.ReceiveBeginPlay` _returnvalue_4)) (stale `self.ReceiveBeginPlay` _returnvalue_4))
        (goto _label)))))

(event `/AstrobotCollectables/BPI_CollectableInterface.Add Friend To Player Inventory`
  (params (aFriend :type "/AstrobotCollectables/Friends/BP_Friend Object Reference") (bDebugMode :type Boolean))
  ;[1 1 1] Add the Friend to the Collectable Inventory
  (`/AstrobotCollectables/Player/BP_CollectableInventory.Add Friend To Player Inventory` (`self.BP_CollectableInventory`) aFriend bDebugMode))

(fn `Get Coin Count`
  (returns (iCoins :type Integer))
  (return 0))

(fn `Get Friend Name`
  (params (iArrayPosition :type Integer))
  (returns (strFriendName :type String))
  (return ""))

(fn `Is Collectable`
  (params (bDebugMode :type Boolean))
  (returns (`is Collectable` :type Boolean))
  (return false))

(fn `UserConstructionScript`)