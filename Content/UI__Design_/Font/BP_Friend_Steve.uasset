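; BP_Friend_Steve is a collectible friend that either of two players picks up by walking into its box trigger.
; On overlap, a per-player timeline holds it in front of the camera of the first Astrobot character found at BeginPlay, whichever player triggered it.
; It plays a wave and the UI manager's collected animation once, then destroys itself.
; A separate BasicAttack function only debug-traces forward and prints the hit actor.
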(event `self.ReceiveBeginPlay`
  (bind _returnvalue (`GameplayStatics.GetActorOfClass` "/Game/Characters/Astrobot/BP_Astrobot_Character.BP_Astrobot_Character_C"))
  (set `self.Character` _returnvalue)
  (bind _returnvalue_2 (`GameplayStatics.GetActorOfClass` "/Game/UI__Design_/BP_UIManager.BP_UIManager_C")))

(event `self.Box.OnComponentBeginOverlap`
  (params (OverlappedComponent :type "PrimitiveComponent Object Reference") (OtherActor :type "Actor Object Reference") (OtherComp :type "PrimitiveComponent Object Reference") (OtherBodyIndex :type Integer) (bFromSweep :type Boolean) (SweepResult :type "HitResult Structure (by ref)"))
  (bind _camera (`/Game/Characters/Astrobot/BP_Astrobot_Character.Camera` (`self.Character`)))
  (bind _camera_2 (`/Game/Characters/Astrobot/BP_Astrobot_Character.Camera` (`self.Character`)))
  (if (== OtherActor (`GameplayStatics.GetPlayerCharacter` 0))
    (`Timeline|Timeline`
      (:`Update`
        (`self.K2_SetActorLocation` (+ (`SceneComponent.K2_GetComponentLocation` _camera) (* (`SceneComponent.GetForwardVector` _camera) 250.0)))
        (`self.K2_SetActorRotation` (`SceneComponent.K2_GetComponentRotation` _camera))
        (`/Engine/EditorBlueprintResources/StandardMacros.DoOnce` false
          (:`Completed`
            (`SkeletalMeshComponent.PlayAnimation` (`self.Mesh`) "/Game/Characters/Astrobot/Animations/Idle/Wave_Both_Arms.Wave_Both_Arms" false)
            (bind _friend_collected (`/Game/UI__Design_/BP_UIManager.Friend Collected` (stale `self.ReceiveBeginPlay` _returnvalue_2)))
            (`/Game/UI__Design_/WBP_FriendRescued.Animation Collected f2` _friend_collected))))
      (:`Finished`
        (`self.K2_DestroyActor`)))
    (elif (== OtherActor (`GameplayStatics.GetPlayerCharacter` 1))
      (`Timeline|Timeline_0`
        (:`Update`
          (`self.K2_SetActorLocation` (+ (`SceneComponent.K2_GetComponentLocation` _camera_2) (* (`SceneComponent.GetForwardVector` _camera_2) 250.0)))
          (`self.K2_SetActorRotation` (`SceneComponent.K2_GetComponentRotation` _camera_2))
          (`/Engine/EditorBlueprintResources/StandardMacros.DoOnce` false
            (:`Completed`
              (`SkeletalMeshComponent.PlayAnimation` (`self.Mesh`) "/Game/Characters/Astrobot/Animations/Idle/Wave_Both_Arms.Wave_Both_Arms" false)
              (`/Game/UI__Design_/WBP_FriendRescued.Animation Collected f2` _friend_collected))))
        (:`Finished`
          (`self.K2_DestroyActor`))))))

(fn `BasicAttack`
  (bind _returnvalue (`SceneComponent.K2_GetComponentLocation` (`self.Mesh`)))
  (bind _outhit (`KismetSystemLibrary.LineTraceSingle` :`Start` (+ _returnvalue (0.0 0.0 2.0)) :`End` (+ (* (`SceneComponent.GetForwardVector` (`self.Mesh`)) 250.0) _returnvalue) :`TraceChannel` "TraceTypeQuery1" :`DrawDebugType` "ForDuration"))
  (`KismetSystemLibrary.PrintString` (`KismetSystemLibrary.GetDisplayName` (`.HitActor` (`GameplayStatics.BreakHitResult` _outhit)))))

(fn `UserConstructionScript`)