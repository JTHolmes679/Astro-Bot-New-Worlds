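; Collectible friend actor (Batman) that the Astrobot character picks up by overlapping its box.
; On overlap, a timeline holds it in front of the player camera, matching its rotation, then destroys it when finished.
; A DoOnce plays the two-arm wave and the third friend's collected animation through the UI manager found at BeginPlay.
; An uncalled BasicAttack function does a debug forward line trace.
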(event `self.ReceiveBeginPlay`
  (bind _returnvalue (`GameplayStatics.GetActorOfClass` "/Game/UI__Design_/BP_UIManager.BP_UIManager_C")))

(event `self.Box.OnComponentBeginOverlap`
  (params (OverlappedComponent :type "PrimitiveComponent Object Reference") (OtherActor :type "Actor Object Reference") (OtherComp :type "PrimitiveComponent Object Reference") (OtherBodyIndex :type Integer) (bFromSweep :type Boolean) (SweepResult :type "HitResult Structure (by ref)"))
  (cast `/Game/Characters/Astrobot/BP_Astrobot_Character` OtherActor)
  (bind _asbp_astrobot_character (cast `/Game/Characters/Astrobot/BP_Astrobot_Character` (`GameplayStatics.GetPlayerPawn` 0)))
  (`Timeline|Timeline`
    (:`Update`
      (bind _camera (`/Game/Characters/Astrobot/BP_Astrobot_Character.Camera` _asbp_astrobot_character))
      (`self.K2_SetActorLocation` (+ (`SceneComponent.K2_GetComponentLocation` _camera) (* (`SceneComponent.GetForwardVector` _camera) 250.0)))
      (`self.K2_SetActorRotation` (`SceneComponent.K2_GetComponentRotation` _camera))
      (`/Engine/EditorBlueprintResources/StandardMacros.DoOnce` false
        (:`Completed`
          (`SkeletalMeshComponent.PlayAnimation` (`self.Mesh`) "/Game/Characters/Astrobot/Animations/Idle/Wave_Both_Arms.Wave_Both_Arms" false)
          (`/Game/UI__Design_/WBP_FriendRescued.Animation Collected f3` (`/Game/UI__Design_/BP_UIManager.Friend Collected` (stale `self.ReceiveBeginPlay` _returnvalue))))))
    (:`Finished`
      (`self.K2_DestroyActor`))))

(fn `BasicAttack`
  (bind _returnvalue (`SceneComponent.K2_GetComponentLocation` (`self.Mesh`)))
  (bind _outhit (`KismetSystemLibrary.LineTraceSingle` :`Start` (+ _returnvalue (0.0 0.0 2.0)) :`End` (+ (* (`SceneComponent.GetForwardVector` (`self.Mesh`)) 250.0) _returnvalue) :`TraceChannel` "TraceTypeQuery1" :`DrawDebugType` "ForDuration"))
  (`KismetSystemLibrary.PrintString` (`KismetSystemLibrary.GetDisplayName` (`.HitActor` (`GameplayStatics.BreakHitResult` _outhit)))))

(fn `UserConstructionScript`)