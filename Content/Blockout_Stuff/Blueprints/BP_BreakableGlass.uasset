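; Breakable glass pane that shatters after a delay when an actor overlaps its trigger box, ignoring other glass panes and fields.
; Shattering enables physics on the Chaos fractured glass, disables mesh collision and spawns a BP_GlassField.
; If rebuilding is allowed, it later spawns a replacement with the same settings, then destroys the field and itself.
; The construction script scales the fractured glass from frame dimensions and sizes the box to the glass mesh.
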(event `self.ReceiveBeginPlay`
  (`parent.ReceiveBeginPlay`)
  ;[1 1 1] Debug mode
  (`SceneComponent.SetHiddenInGame` (`self.Box`) (not (`self.bDebugMode`)) false))

(event `self.Box.OnComponentBeginOverlap`
  (params (OverlappedComponent :type "PrimitiveComponent Object Reference") (OtherActor :type "Actor Object Reference") (OtherComp :type "PrimitiveComponent Object Reference") (OtherBodyIndex :type Integer) (bFromSweep :type Boolean) (SweepResult :type "HitResult Structure (by ref)"))
  (bind _returnvalue (`GameplayStatics.GetObjectClass` OtherActor))
  ;[1 1 1] Collision detection
  ;;[1 1 1] Prevent collisions when respawning
  (if (and (!= _returnvalue "BP_BreakableGlass_C") (!= _returnvalue "/Game/Blockout_Stuff/Blueprints/BP_GlassField.BP_GlassField_C"))
    (`KismetSystemLibrary.PrintString` "Collision" (`self.bDebugMode`))
    ;;[1 1 1] Restore Glass
    (`KismetSystemLibrary.Delay` (`self.fShatterDelay`))
    (`self.Shatter Glass`)
    ;;[1 1 1] Rebuild Glass
    (if (`self.bCanRebuild`)
      (`KismetSystemLibrary.Delay` (`self.fRebuildDelay`))
      (`self.Restore Glass`)
      (else
        (`KismetSystemLibrary.PrintString` "Cannot Restore" (`self.bDebugMode`))))))

(event `Shatter Glass`
  ;[1 1 1] Activate Physics for the Chaos Geometry Collision
  (`PrimitiveComponent.SetSimulatePhysics` (`self.Shattered Glass`) true)
  (`PrimitiveComponent.SetCollisionEnabled` (`self.glassmesh`) "NoCollision")
  (`KismetSystemLibrary.PrintString` "Shatter" (`self.bDebugMode`))
  (bind _returnvalue (`|SpawnActorFromClass` "/Game/Blockout_Stuff/Blueprints/BP_GlassField.BP_GlassField_C" (`self.GetTransform`) "Undefined" "MultiplyWithRoot" null null))
  (set `self.aGlassField` _returnvalue))

(event `Restore Glass`
  ;[1 1 1] Spawn in a new glass actor and destroy this actor
  (bind _returnvalue (`|SpawnActorFromClass` "BP_BreakableGlass_C" (`self.GetTransform`) "Undefined" "MultiplyWithRoot" null (`self.fShatterDelay`) (`self.fRebuildDelay`) (`self.bCanRebuild`) true (`self.FrameWidth`) (`self.FrameHeight`) null))
  (`KismetSystemLibrary.PrintString` "Restored" (`self.bDebugMode`))
  (`self.K2_DestroyActor` (`self.aGlassField`))
  (`self.K2_DestroyActor`))

(fn `UserConstructionScript`
  (bind _shattered_glass (`self.Shattered Glass`))
  (bind _glassmesh (`self.glassmesh`))
  (bind (_min _max) (`StaticMeshComponent.GetLocalBounds` _glassmesh))
  (bind (_relativescale3d_x _relativescale3d_y) (`KismetMathLibrary.BreakVector` (`SceneComponent.RelativeScale3D` _glassmesh)))
  (bind (_returnvalue_x _returnvalue_y) (`KismetMathLibrary.BreakVector` (+ (`SceneComponent.RelativeScale3D` _shattered_glass) (`KismetMathLibrary.MakeVector` (/ (`self.FrameWidth`) (`self.glass length`)) (/ (`self.FrameHeight`) (`self.glass length`))))))
  ;[1 1 1] Set Mesh Scale
  (`parent.UserConstructionScript`)
  (`SceneComponent.SetRelativeScale3D` _shattered_glass (`KismetMathLibrary.MakeVector` _returnvalue_x _returnvalue_y 1.0))
  ;[1 1 1] Set Collision Box scale
  (`BoxComponent.SetBoxExtent` (`self.Box`) (`KismetMathLibrary.MakeVector` (* (.x _max) _relativescale3d_x) (* (.y _max) _relativescale3d_y) 32.0) true))