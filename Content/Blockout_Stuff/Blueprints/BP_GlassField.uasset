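; BP_GlassField is a one-shot Chaos field actor that, judging by its name, shatters glass Geometry Collections.
; On BeginPlay it applies external cluster strain through a linear radial falloff sized and centered on its Sphere component.
; It then applies radial linear and angular velocity from just above the sphere center, using that falloff to cull outside the radius.
; The actor destroys itself immediately afterward.
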(event `self.ReceiveBeginPlay`
  (bind _sphere (`self.Sphere`))
  (bind _returnvalue (`SceneComponent.K2_GetComponentLocation` _sphere))
  (bind _returnvalue_2 (`RadialFalloff.SetRadialFalloff` (`self.RadialFalloff`) 5550000.0 0.0 1.0 50000.0 (`SphereComponent.GetScaledSphereRadius` _sphere) _returnvalue "Field_Falloff_Linear"))
  (bind _returnvalue_3 (+ _returnvalue (0.0 0.0 100.0)))
  (`FieldSystemComponent.ApplyPhysicsField` (`self.FieldSystemComponent`) true "Field_ExternalClusterStrain" null _returnvalue_2)
  (`FieldSystemComponent.ApplyPhysicsField` (`self.FieldSystemComponent`) true "Field_LinearVelocity" null (`CullingField.SetCullingField` (`self.CullingField`) _returnvalue_2 (`RadialVector.SetRadialVector` (`self.RadialVector`) 1500.0 _returnvalue_3) "Field_Culling_Outside"))
  (`FieldSystemComponent.ApplyPhysicsField` (`self.FieldSystemComponent`) true "Field_AngularVelociy" null (`CullingField.SetCullingField` (`self.CullingField`) _returnvalue_2 (`RadialVector.SetRadialVector` (`self.RadialVector`) 1.0 _returnvalue_3) "Field_Culling_Outside"))
  (`self.K2_DestroyActor`))

(fn `UserConstructionScript`)