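; BP_Platform is a moving platform that shuttles back and forth between two end points once its Activate event is called.
; Activate runs an endless latent loop, using MoveComponentTo to slide the Cube component to the relative location of End, then back to Start.
; Speed sets the duration of each move rather than a velocity, and StaticTime sets the pause after each one.
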(event `/Game/Platform-Kit/BI_Activation.Activate`
  ;[1 1 1] The loop of having the platofrom move between the 2 end points
  (`KismetSystemLibrary.MoveComponentTo` (`self.Cube`) (`SceneComponent.RelativeLocation` (`self.End`)) (struct) false false (`self.Speed`) :!label _label)
  (`KismetSystemLibrary.Delay` (`self.StaticTime`))
  (`KismetSystemLibrary.MoveComponentTo` (`self.Cube`) (`SceneComponent.RelativeLocation` (`self.Start`)) (struct) false false (`self.Speed`))
  (`KismetSystemLibrary.Delay` (`self.StaticTime`))
  (goto _label))

(fn `UserConstructionScript`)