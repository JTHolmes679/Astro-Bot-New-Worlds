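; BP_Controller is a control actor that tells a linked controllable platform which direction to move.
; Its Activate event converts a direction enum (left, right, forward, backward, up, down) into an axis unit vector, with forward mapped to negative Y.
; It then passes that vector to PlatformToControl through an ActivateControllablePlatformMessage call, leaving movement to the platform.
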(event `/Game/Platform-Kit/BI_Activation.Activate(ControllablePlatform)`
  (params (MovementDirectionVector :type "Vector Structure"))
  (switch `/Game/Platform-Kit/Controllable_Platform/ENUM_MovementDirection` (`self.MovementDirtectionType`)
    (:`NewEnumerator0`
      (set `self.MovementDirectionVector` (-1.0 0.0 0.0)))
    (:`NewEnumerator1`
      (set `self.MovementDirectionVector` (1.0 0.0 0.0)))
    (:`NewEnumerator2`
      (set `self.MovementDirectionVector` (0.0 -1.0 0.0)))
    (:`NewEnumerator3`
      (set `self.MovementDirectionVector` (0.0 1.0 0.0)))
    (:`NewEnumerator4`
      (set `self.MovementDirectionVector` (0.0 0.0 1.0)))
    (:`NewEnumerator5`
      (set `self.MovementDirectionVector` (0.0 0.0 -1.0))))
  (message `/Game/Platform-Kit/BI_Activation.Activate(ControllablePlatform)` (`self.Platform To Control`) (`self.MovementDirectionVector`)))

(fn `UserConstructionScript`)