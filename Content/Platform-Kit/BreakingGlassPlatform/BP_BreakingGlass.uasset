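; Breakable glass platform built on a Chaos Geometry Collection, which shatters and is later respawned through the player character.
; On BeginPlay it saves its transform and puts the collection to sleep.
; A Chaos break event makes the collection dynamic and disables its collision.
; After a short delay it hands its transform, respawn delay and anchor fields to the player character via GlassRespawnMessage, then destroys itself.
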(event `self.ReceiveBeginPlay`
  (set `self.Platform Location` (`self.GetTransform`))
  (`PrimitiveComponent.PutRigidBodyToSleep` (`self.GeometryCollection`) "None"))

(event `self.GeometryCollection.OnChaosBreakEvent`
  (params (BreakEvent :type "ChaosBreakEvent Structure (by ref)"))
  (bind _geometrycollection (`self.GeometryCollection`))
  (set `GeometryCollectionComponent.ObjectType` "Chaos_Object_Dynamic" _geometrycollection)
  (`PrimitiveComponent.SetCollisionEnabled` _geometrycollection "NoCollision")
  (`KismetSystemLibrary.Delay` 2.0)
  (message `/Game/Platform-Kit/BreakingGlassPlatform/BI_GlassRespawn.Glass Respawn` (`GameplayStatics.GetPlayerCharacter` 0) (`self.Platform Location`) (`self.DelayBeforeRespawn`) (`GeometryCollectionComponent.InitializationFields` (`self.GeometryCollection`)))
  (`self.K2_DestroyActor`))

(fn `UserConstructionScript`)