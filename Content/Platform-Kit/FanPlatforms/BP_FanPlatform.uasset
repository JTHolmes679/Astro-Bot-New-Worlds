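; BP_FanPlatform is a fan platform that pushes the player along its arrow direction while they are inside its airflow volume.
; AirFlow overlap activates the fan when it is always on, otherwise copies the linked fan switch's state at entry, and leaving deactivates it.
; Every Tick sends the player character either FanUpMessage with the Arrow's forward vector or FanDownMessage, leaving the movement response to the character.
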(event `self.ReceiveTick`
  (params (DeltaSeconds :type "Float (single-precision)"))
  ;[1 1 1] Getting direction player goes in
  (if (`self.B_FanActive`)
    (message `/Game/Platform-Kit/BI_Activation.Fan_Up` (`GameplayStatics.GetPlayerCharacter` 0) (`SceneComponent.GetForwardVector` (`self.Arrow`)))
    (else
      (message `/Game/Platform-Kit/BI_Activation.Fan_Down` (`GameplayStatics.GetPlayerCharacter` 0)))))

(event `self.AirFlow.OnComponentBeginOverlap`
  (params (OverlappedComponent :type "PrimitiveComponent Object Reference") (OtherActor :type "Actor Object Reference") (OtherComp :type "PrimitiveComponent Object Reference") (OtherBodyIndex :type Integer) (bFromSweep :type Boolean) (SweepResult :type "HitResult Structure (by ref)"))
  ;[1 1 1] Fan Activation on overlap
  (if (== OtherActor (`GameplayStatics.GetPlayerCharacter` 0))
    (if (`self.B_FanAlwaysOn`)
      (set `self.B_FanActive` true)
      (else
        (set `self.B_FanActive` (`/Game/Platform-Kit/FanPlatforms/BP_FanSwitch.B_FanActivated` (`self.BP_FanSwitch`)))))))

(event `self.AirFlow.OnComponentEndOverlap`
  (params (OverlappedComponent :type "PrimitiveComponent Object Reference") (OtherActor :type "Actor Object Reference") (OtherComp :type "PrimitiveComponent Object Reference") (OtherBodyIndex :type Integer))
  ;[1 1 1] Fan Activation on overlap
  (if (== OtherActor (`GameplayStatics.GetPlayerCharacter` 0))
    (set `self.B_FanActive` false)))

(fn `UserConstructionScript`)